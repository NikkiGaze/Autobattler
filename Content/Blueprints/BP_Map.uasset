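; BP_Map is a map actor that builds a Width by Height hexagonal-style tile grid from an Instanced Static Mesh.
; The Construction Script runs nested loops over rows and columns, adding one instance per tile, spaced by TileRadius.
; A FlipFlop shifts alternate rows back half a tile in X, while sqrt(3)/2 scales the row spacing in Y.
; The event graph holds only disabled placeholder events.
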(fn `UserConstructionScript`
  (bind _output_get (set `self.HeghtOffset` (/ (`KismetMathLibrary.Sqrt` 3.0) 2.0)))
  (for _index (range (+ (`self.Height`) 1))
    (`/Engine/EditorBlueprintResources/StandardMacros.FlipFlop`
      (:`A`
        (set `self.TileOffset` 0.0))
      (:`B`
        (set `self.TileOffset` (* (`self.TileRadius`) -0.5))))
    (for _index_2 (range (+ (`self.Width`) 1))
      (`InstancedStaticMeshComponent.AddInstance` (`self.InstancedStaticMesh`) (`KismetMathLibrary.MakeTransform` (`KismetMathLibrary.MakeVector` (+ (* _index_2 (`self.TileRadius`)) (`self.TileOffset`)) (* (* _index (`self.TileRadius`)) _output_get))) false))))